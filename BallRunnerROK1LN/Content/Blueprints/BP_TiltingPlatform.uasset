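; Tilting platform that rolls its Cube while a BP_Ball_01 is inside its trigger zone and levels it afterwards.
; TriggerZone begin and end overlaps cast the other actor's class to BP_Ball_01 and set or clear IsTilting.
; Tick interpolates the Cube's relative roll toward TilyAngle or back to zero with FInterpTo, using TiltSpeed and delta time scaled by DeltaMultiplier, while holding pitch and yaw at zero.
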(event `self.TriggerZone.OnComponentBeginOverlap`
  (params (OverlappedComponent :type "PrimitiveComponent Object Reference") (OtherActor :type "Actor Object Reference") (OtherComp :type "PrimitiveComponent Object Reference") (OtherBodyIndex :type Integer) (bFromSweep :type Boolean) (SweepResult :type "HitResult Structure (by ref)"))
  (bind _asbp_ball_01 (castclass `/Game/Blueprints/BP_Ball_01` (`GameplayStatics.GetObjectClass` OtherActor)))
  (set `self.IsTilting` true))

(event `self.TriggerZone.OnComponentEndOverlap`
  (params (OverlappedComponent :type "PrimitiveComponent Object Reference") (OtherActor :type "Actor Object Reference") (OtherComp :type "PrimitiveComponent Object Reference") (OtherBodyIndex :type Integer))
  (bind _asbp_ball_01 (castclass `/Game/Blueprints/BP_Ball_01` (`GameplayStatics.GetObjectClass` OtherActor)))
  (set `self.IsTilting` false))

(event `self.ReceiveTick`
  (params (DeltaSeconds :type "Float (single-precision)"))
  (bind _tiltspeed (`self.TiltSpeed`))
  (bind _cube (`self.Cube`))
  (bind _returnvalue (* (`self.DeltaMultiplier`) DeltaSeconds))
  (bind _roll (.roll (`SceneComponent.RelativeRotation` (`self.Cube`))))
  (if (`self.IsTilting`)
    (`SceneComponent.K2_SetRelativeRotation` _cube (`KismetMathLibrary.MakeRotator` (`KismetMathLibrary.FInterpTo` _roll (`self.TilyAngle`) _returnvalue _tiltspeed)) false false)
    (else
      (`SceneComponent.K2_SetRelativeRotation` _cube (`KismetMathLibrary.MakeRotator` (`KismetMathLibrary.FInterpTo` _roll 0.0 _returnvalue _tiltspeed)) false false))))

(fn `UserConstructionScript`)