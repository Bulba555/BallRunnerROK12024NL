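; BP_WinVolume_01 is a level-exit trigger that completes the level when the player overlaps its box and all crystals are collected.
; Any remaining BP_Crystal_01 or BP_Crystal_02 actor blocks completion with a Polish debug message.
; Otherwise it plays a teleport sound, blacks out the camera and, after a short delay, opens the next level in TabLevelNames01.
; On the final level it only prints a message.
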(event `self.Box.OnComponentBeginOverlap`
  (params (OverlappedComponent :type "PrimitiveComponent Object Reference") (OtherActor :type "Actor Object Reference") (OtherComp :type "PrimitiveComponent Object Reference") (OtherBodyIndex :type Integer) (bFromSweep :type Boolean) (SweepResult :type "HitResult Structure (by ref)"))
  (`/Game/Library/ML_Validation_01.IsPlayer` OtherActor
    (:`true`
      (bind _returnvalue (`self.CheckAnyCrystals`))
      (if _returnvalue
        (`KismetSystemLibrary.PrintString` "Nie zebrano wszystkich krystalow" true true (struct :`R` 0.954861 :`G` 0.049838 :`B` 0.005495 :`A` 1.0))
        (else
          (`GameplayStatics.SpawnSound2D` "/Game/Music/Teleport_cue.Teleport_cue" 1.0 1.0 0.0 null)
          (`PlayerCameraManager.StartCameraFade` (`GameplayStatics.GetPlayerCameraManager` 0) 2.0 2.0 5.0 (struct :`A` 1.0) false true)
          (`KismetSystemLibrary.Delay` 0.5)
          (`self.CompleteLevel`))))))

(fn `CheckAnyCrystals`
  (returns (ReturnValue :type Boolean))
  (bind _outactors (`GameplayStatics.GetAllActorsOfClass` "/Game/Blueprints/BP_Crystal_01.BP_Crystal_01_C"))
  (bind _outactors_2 (`GameplayStatics.GetAllActorsOfClass` "/Game/Blueprints/BP_Crystal_02.BP_Crystal_02_C"))
  (return (or (> (`KismetArrayLibrary.Array_Length` _outactors_2) 0) (> (`KismetArrayLibrary.Array_Length` _outactors) 0))))

(fn `CompleteLevel`
  (if (`self.IsFinalLevel`)
    (`KismetSystemLibrary.PrintString` "To jest ostatni poziom")
    (else
      (`self.LoadNextLevel`))))

(fn `GetCurrentLevelIndex`
  (returns (LevelIndex :type Integer))
  (bind _returnvalue (`GameplayStatics.GetCurrentLevelName` true))
  (return (`KismetArrayLibrary.Array_Find` (`self.Tab_LevelNames_01`) _returnvalue)))

(fn `GetNextLevelName`
  (returns (NextLevelName :type String))
  (return (`|GetArrayItem` (`self.Tab_LevelNames_01`) (+ (`self.GetCurrentLevelIndex`) 1))))

(fn `IsFinalLevel`
  (returns (ReturnValue :type Boolean))
  (return (== (`KismetArrayLibrary.Array_LastIndex` (`self.Tab_LevelNames_01`)) (`self.GetCurrentLevelIndex`))))

(fn `LoadNextLevel`
  (`GameplayStatics.OpenLevel` (`KismetStringLibrary.Conv_StringToName` (`self.GetNextLevelName`))))

(fn `UserConstructionScript`)